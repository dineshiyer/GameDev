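; Saturn actor that moves its Sphere along a horizontal elliptical path at a fixed height.
; A looping fast timer started on BeginPlay calls Draw Ellipse, computing position from game time, Speed, Width and Height with sine and cosine.
; Each call also spawns a non-auto-destroying emitter, using that relative offset as a world location.
; The construction script applies the Material; a Timeline-based movement path is left unconnected.
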(event EventBeginPlay
  (Utilities|Time|SetTimerbyFunctionName 0 "Draw  Ellipse" 0.01 true))

(event EventActorBeginOverlap
  (params (OtherActor :type Actor%20Object%20Reference)))

(event EventTick
  (params (DeltaSeconds :type Float%20%28single-precision%29)))

(fn ConstructionScript
  (Rendering|Material|SetMaterial (Variables|Default|GetSphere) 0 (Variables|Default|GetMaterial)))

(fn DrawEllipse
  (bind _returnvalue (Utilities|Time|GetGameTimeinSeconds))
  (bind _width (Variables|Default|GetWidth))
  (bind _height (Variables|Default|GetHeight))
  (bind _speed (Variables|Default|GetSpeed))
  (bind _returnvalue_2 (* _returnvalue _speed))
  (bind _returnvalue_3 (Math|Trig|Sin(Degrees) _returnvalue_2))
  (bind _returnvalue_4 (Math|Trig|Cos(Degrees) _returnvalue_2))
  (bind _returnvalue_5 (* _returnvalue_4 _height))
  (bind _returnvalue_6 (* _returnvalue_3 _width))
  (bind _returnvalue_7 (Math|Vector|MakeVector _returnvalue_6 _returnvalue_5 152.199432))
  (Transformation|SetRelativeLocation (Variables|Default|GetSphere) _returnvalue_7 false)
  (Effects|SpawnEmitteratLocation "/Game/StarterContent/Particles/SOmw.SOmw" _returnvalue_7 "0.000000,90.000000,0.000000" false))