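; Planet actor that orbits and spins, and opens an info card when clicked.
; A looping timer, rather than Tick, sets absolute yaw from game time on the Pivot for revolution and on the planet component for rotation.
; The construction script applies a dynamic instance of the configured planet material.
; Clicking the planet pauses the game, adds the InfoCardName widget to the viewport and shows the mouse cursor.
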(event OnClicked(PLanet)
  (params (TouchedComponent :type Primitive%20Component%20Object%20Reference))
  (bind _returnvalue (Game|GetPlayerController 0))
  (Game|SetGamePaused true)
  (bind _returnvalue_2 (UserInterface|CreateWidget (Variables|Default|GetInfoCardName) _returnvalue))
  (UserInterface|Viewport|AddtoViewport _returnvalue_2 0)
  (Variables|/Script/Engine.PlayerController|SetbShowMouseCursor _returnvalue true))

(event EventBeginPlay
  (Utilities|Time|SetTimerbyFunctionName 0 "PlanetRotation&Revolution" 0.1 true))

(event Collision|EventActorBeginOverlap
  (params (OtherActor :type Actor%20Object%20Reference)))

(event EventTick
  (params (DeltaSeconds :type Float%20%28single-precision%29)))

(fn ConstructionScript
  (Rendering|Material|CreateDynamicMaterialInstance (Variables|Default|GetPLanet) 0 (Variables|Default|GetPlanetMaterial) :!class /Script/Engine.PrimitiveComponent))

(fn PlanetRotation&Revolution
  (Utilities|FlowControl|Sequence
    (:then_0
      (Transformation|SetWorldRotation (Variables|Default|GetPivot) (Class|KismetMathLibrary|MakeRot 0.0 (* (Variables|Default|GetBaseSpeed) (Utilities|Time|GetGameTimeinSeconds)) 0.0) false))
    (:then_1
      (Transformation|SetWorldRotation (Variables|Default|GetPLanet) (Class|KismetMathLibrary|MakeRot 0.0 (* (Utilities|Time|GetGameTimeinSeconds) (Variables|Default|GetDayTime)) 0.0) false))))